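; Enemy spawner actor that places one enemy of a configured class at its SpawnPoint.
; On BeginPlay it spawns the enemy, destroys its own SkeletalMesh component and binds the spawn event to BP_GameMode's enemy respawn hook.
; Each spawn destroys any surviving previous enemy, then hands the new one its starting transform and location.
; The Box overlap event is empty.
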(event OnComponentBeginOverlap(Box)
  (params (OverlappedComponent :type Primitive%20Component%20Object%20Reference) (OtherActor :type Actor%20Object%20Reference) (OtherComp :type Primitive%20Component%20Object%20Reference) (OtherBodyIndex :type Integer) (bFromSweep :type Boolean) (SweepResult :type Hit%20Result%20Structure%20%28by%20ref%29)))

(event Custom|SpawnEnemy
  (bind _spawn_point (Variables|Default|Getspawn%20point))
  (Utilities|IsValid (Variables|Default|GetEnemySpawned)
    (:Is%20Valid
      (Actor|DestroyActor (Variables|Default|GetEnemySpawned)))
    (:Is%20Not%20Valid
      _))
  (bind _returnvalue (Game|SpawnActorfromClass (Variables|Default|GetEnemy) (Transformation|GetWorldTransform (Variables|Default|Getspawn%20point)) "Undefined" "MultiplyWithRoot" 0 0))
  (bind _output_get (Variables|Default|SetEnemySpawned _returnvalue))
  (Variables|/Game/AI/BP_EnemyAI.BP_EnemyAI_C|SetstartingTransform _output_get (Transformation|GetWorldTransform _spawn_point))
  (Variables|/Game/AI/BP_EnemyAI.BP_EnemyAI_C|SetStartLocation _output_get (Transformation|GetWorldLocation _spawn_point)))

(event EventBeginPlay
  (CallFunction|SpawnEnemy)
  (Components|DestroyComponent (Variables|Default|GetSkeletalMesh))
  (bind _asbp_game_mode (Utilities|Casting|CastToBP_GameMode (Game|GetGameMode)))
  (EventDispatchers|BindEventtoRespawnEnemies _asbp_game_mode (delegate Custom|SpawnEnemy)))

(event Collision|EventActorBeginOverlap
  (params (OtherActor :type Actor%20Object%20Reference)))

(event EventTick
  (params (DeltaSeconds :type Float%20%28single-precision%29)))

(fn ConstructionScript)
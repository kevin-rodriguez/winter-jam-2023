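; Enemy AI pawn that chases the player after spotting them and triggers game over on catching them.
; PawnSensing sets a seeing flag, and Tick steers straight at the player, clearing the flag beyond a fixed range.
; Within attack distance, it calls GameOver on BP_Michi and BP_GameMode and shows a game-over screen.
; The AIMoveTo-based FollowPlayer event and the return-to-start, respawn and debug nodes are left unused.
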(event OnSeePawn(PawnSensing)
  (params (Pawn :type Pawn%20Object%20Reference))
  ;[1 1 1] Enemy Sees Player
  (Variables|Default|SetisSeeingPlayer? true))

(event Custom|FollowPlayer
  (bind _returnvalue (Game|GetPlayerCharacter 0))
  ;[1 1 1] Follow Player
  (if (Variables|Default|GetisSeeingPlayer?)
    (AI|AIMoveTo self "0, 0, 0" _returnvalue 2.0 false
      (:OnSuccess
        (if (< (Transformation|GetDistanceTo self _returnvalue) (Variables|Default|GetattackDistance))
          (bind _asbp_michi (Utilities|Casting|CastToBP_Michi _returnvalue))
          (Default|GameOver _asbp_michi)
          (bind _asbp_game_mode (Utilities|Casting|CastToBP_GameMode (Game|GetGameMode)))
          (Default|GameOver _asbp_game_mode)
          (Default|GameOverScreens (Variables|/Game/BP_GameMode.BP_GameMode_C|GetGameOverWidget _asbp_game_mode) "NewEnumerator2"))))))

(event EventBeginPlay)

(event Collision|EventActorBeginOverlap
  (params (OtherActor :type Actor%20Object%20Reference)))

(event EventTick
  (params (DeltaSeconds :type Float%20%28single-precision%29))
  (bind _returnvalue (Game|GetPlayerCharacter 0))
  (bind _self self)
  (bind _returnvalue_2 (Transformation|GetDistanceTo _self _returnvalue))
  (if (Variables|Default|GetisSeeingPlayer?)
    (Pawn|Input|AddMovementInput (Math|Vector|Normalize (- (Transformation|GetActorLocation (Game|GetPlayerCharacter 0)) (Transformation|GetActorLocation))) (* DeltaSeconds 6e+01) false)
    (if (< _returnvalue_2 (Variables|Default|GetattackDistance))
      (bind _asbp_michi (Utilities|Casting|CastToBP_Michi _returnvalue))
      (Default|GameOver _asbp_michi)
      (bind _asbp_game_mode (Utilities|Casting|CastToBP_GameMode (Game|GetGameMode)))
      (Default|GameOver _asbp_game_mode)
      (Default|GameOverScreens (Variables|/Game/BP_GameMode.BP_GameMode_C|GetGameOverWidget _asbp_game_mode) "NewEnumerator2")
      (elif (not (< _returnvalue_2 3e+02))
        (Variables|Default|SetisSeeingPlayer? false)))))

(fn ConstructionScript)
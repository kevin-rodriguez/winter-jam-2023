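; Checkpoint actor that marks where the player character respawns.
; When a BP_Character overlaps its Box, it caches that character and registers itself as the character's CheckpointBP.
; EventRespawn spawns a new actor of the cached character's class at the RespawnPoint location with a fixed rotation.
; An older SaveGame_OBJ approach that stored the checkpoint's location as PlayerLocation remains in the graph but is disconnected.
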(event OnComponentBeginOverlap(Box)
  (params (OverlappedComponent :type Primitive%20Component%20Object%20Reference) (OtherActor :type Actor%20Object%20Reference) (OtherComp :type Primitive%20Component%20Object%20Reference) (OtherBodyIndex :type Integer) (bFromSweep :type Boolean) (SweepResult :type Hit%20Result%20Structure%20%28by%20ref%29))
  (bind _asbp_character (Utilities|Casting|CastToBP_Character OtherActor))
  (Variables|Default|SetBP_character _asbp_character)
  (Variables|/Game/Character/Blueprints/BP_Character.BP_Character_C|SetCheckpoint_BP _asbp_character self))

(event Custom|EventRespawn
  (Game|SpawnActorfromClass (Utilities|GetClass (Variables|Default|GetBP_character)) (Math|Transform|MakeTransform (Transformation|GetWorldLocation (Variables|Default|GetRespawnPoint)) "0.000000,-180.000000,0.000000") "Undefined" "MultiplyWithRoot" 0 0))

(event EventBeginPlay)

(event Collision|EventActorBeginOverlap
  (params (OtherActor :type Actor%20Object%20Reference)))

(event EventTick
  (params (DeltaSeconds :type Float%20%28single-precision%29)))

(fn ConstructionScript)
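; Game mode that starts the level's audio and handles game over.
; BeginPlay applies a sound mix override, plays 2D music and ambience, hides the cursor and gives every BP_EnemyAI the same hardcoded starting transform, despite the "Save Dogs Locations" label.
; GameOver calls RespawnEnemies, disables character input and shows the WB_GameOver widget.
; EnablePlayerInput restores input on the stored player pawn, while DisablePlayerInput is an empty stub.
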(event Custom|Play%20Background%20Music
  (bind _returnvalue (Audio|CreateSound2D "/Game/Musica/Musica/Explorar_SViento.Explorar_SViento" 1.0 1.0 0.0 0))
  (Audio|Components|Audio|Play _returnvalue 0.0))

(event Custom|Play%20Ambience%20Sound
  (bind _returnvalue (Audio|CreateSound2D "/Game/Musica/Musica/Ambiente__Pjaros.Ambiente__Pjaros" 0.5 1.0 0.0 0))
  (Audio|Components|Audio|Play _returnvalue 0.0))

(event EventBeginPlay
  (Audio|SetSoundMixClassOverride "/Game/Musica/SX_Level1.SX_Level1" "/Game/Musica/SClass_MusicaFondo.SClass_MusicaFondo" 1.0 1.0 1.0 true)
  (Variables|Default|SetCharacter (Game|Player|GetPlayerPawn 0))
  (CallFunction|PlayBackgroundMusic)
  (CallFunction|PlayAmbienceSound)
  ;[1 1 1] Save Dogs Locations
  (bind _outactors (Actor|GetAllActorsOfClass "/Game/AI/BP_EnemyAI.BP_EnemyAI_C"))
  (for _array_element _outactors
    (Variables|/Game/AI/BP_EnemyAI.BP_EnemyAI_C|SetstartingTransform _array_element (Math|Transform|MakeTransform "3800.000000,10238.000000,-8.000000" "0.000000,-180.000000,0.000000"))
    (Variables|/Script/Engine.PlayerController|SetbShowMouseCursor (Game|GetPlayerController 0) false)))

(event EventTick
  (params (DeltaSeconds :type Float%20%28single-precision%29)))

(fn ConstructionScript)

(fn GameOver
  (Default|CallRespawnEnemies)
  (Input|DisableInput (Variables|Default|GetBP_Character) (Game|GetPlayerController 0))
  (bind _returnvalue (UserInterface|CreateWidget "/Game/Widgets/WB_GameOver.WB_GameOver_C"))
  (bind _output_get (Variables|Default|SetGameOverWidget _returnvalue))
  (UserInterface|Viewport|AddtoViewport _output_get 0))

(fn EnablePlayerInput
  (Input|EnableInput (Variables|Default|GetCharacter) (Game|GetPlayerController 0)))

(fn DisablePlayerInput)
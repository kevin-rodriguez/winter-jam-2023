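; BP_Pescador is a fisherman hazard that calls GameOver on BP_Character when the character overlaps its Collision component.
; On BeginPlay, ChangeState plays the Vista timeline from the start or in reverse from the end, depending on the Reposo flag.
; The timeline lerps Collision's relative location along local X between two offsets, sweeping the detection area across the fisherman without physics sweep.
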(event OnComponentBeginOverlap(Collision)
  (params (OverlappedComponent :type Primitive%20Component%20Object%20Reference) (OtherActor :type Actor%20Object%20Reference) (OtherComp :type Primitive%20Component%20Object%20Reference) (OtherBodyIndex :type Integer) (bFromSweep :type Boolean) (SweepResult :type Hit%20Result%20Structure%20%28by%20ref%29))
  (bind _asbp_character (Utilities|Casting|CastToBP_Character OtherActor))
  (Default|GameOver _asbp_character))

(event Custom|ChangeState
  (if (Variables|Default|GetbReposo?)
    (bind _vista (Timeline|Vista PlayFromStart)
      (:Update
        (Transformation|SetRelativeLocation (Variables|Default|GetCollision) (Math|Vector|Lerp(Vector) "-135.000000,0.000000,0.000000" "135.000000,0.000000,0.000000" _vista) false false)))
    (else
      (Timeline|Vista ReverseFromEnd))))

(event EventBeginPlay
  (CallFunction|ChangeState))

(event Collision|EventActorBeginOverlap
  (params (OtherActor :type Actor%20Object%20Reference)))

(event EventTick
  (params (DeltaSeconds :type Float%20%28single-precision%29)))

(fn ConstructionScript)